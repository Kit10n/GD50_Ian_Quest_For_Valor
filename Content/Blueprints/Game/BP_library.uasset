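; BP_library is a shared helper Blueprint for quest marker lookup and item pickup feedback.
; The active quest marker getter returns the first element of the markers message obtained from the game instance.
; Pickup feedback switches on the target's pickup type to choose a particle and sound, then spawns both at the target's location.
; Only potions and keys have effects assigned; gold and gems are set to none.
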(fn FGetActiveQuestMarker
  (bind _activemarkers (Class|QuestMarkerInterface|GetMarkers(Message) (Game|GetGameInstance)))
  (return (Utilities|Array|Get(acopy) _activemarkers)))

(fn FPickupFeedback
  (params (Target :type Quest%20Pickup%20Object%20Reference))
  (bind _returnvalue (Transformation|GetActorLocation Target))
  ;[1 1 1] Spawn particles and audio when the player picks up an item
  (switch Utilities|FlowControl|Switch|SwitchonEnum_PickupTypes (Variables|/Game/Blueprints/Ingredients/QuestPickup.QuestPickup_C|GetPickupType Target)
    (:NewEnumerator0
      (LocalVariables|Setv_particleEffect "/Game/Effects/Particles/Systems/P_Loot_Pickup.P_Loot_Pickup")
      (LocalVariables|Setv_sound "/Game/Audio/SFX/General_GetResources_01.General_GetResources_01"))
    (:NewEnumerator1
      (LocalVariables|Setv_particleEffect 0)
      (LocalVariables|Setv_sound 0))
    (:NewEnumerator2
      (LocalVariables|Setv_particleEffect "/Game/Effects/Particles/Systems/P_Loot_Pickup.P_Loot_Pickup")
      (LocalVariables|Setv_sound "/Game/Audio/SFX/General_GetResources_01.General_GetResources_01"))
    (:NewEnumerator4
      (LocalVariables|Setv_particleEffect 0)
      (LocalVariables|Setv_sound 0)))
  (Effects|SpawnEmitteratLocation 0 (LocalVariables|Getv_particleEffect) _returnvalue)
  (Audio|PlaySoundatLocation 0 (LocalVariables|Getv_sound) _returnvalue))