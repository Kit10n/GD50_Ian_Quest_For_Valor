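; Placeholder beat marker that shows configurable text while the Juno quest character stands inside its trigger box.
; The construction script applies exposed variables to the box extent and to the text's content, color, size and relative location.
; BeginPlay and Juno's begin and end overlaps share one FlipFlop that toggles the text's hidden state, starting hidden rather than setting visibility explicitly per event.
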(event OnComponentBeginOverlap(Trigger)
  (params (OverlappedComponent :type Primitive%20Component%20Object%20Reference) (OtherActor :type Actor%20Object%20Reference) (OtherComp :type Primitive%20Component%20Object%20Reference) (OtherBodyIndex :type Integer) (bFromSweep :type Boolean) (SweepResult :type Hit%20Result%20Structure%20%28by%20ref%29))
  (Utilities|Casting|CastToQuestCharacter_Juno OtherActor)
  (bind _isa (Utilities|FlowControl|FlipFlop)
    (:A
      _)
    (:B
      _))
  (Development|SetHiddeninGame (Variables|Default|GetPlaceholder) _isa false))

(event OnComponentEndOverlap(Trigger)
  (params (OverlappedComponent :type Primitive%20Component%20Object%20Reference) (OtherActor :type Actor%20Object%20Reference) (OtherComp :type Primitive%20Component%20Object%20Reference) (OtherBodyIndex :type Integer))
  (Utilities|Casting|CastToQuestCharacter_Juno OtherActor)
  (bind _isa (Utilities|FlowControl|FlipFlop)
    (:A
      _)
    (:B
      _))
  (Development|SetHiddeninGame (Variables|Default|GetPlaceholder) _isa false))

(event EventBeginPlay
  (bind _isa (Utilities|FlowControl|FlipFlop)
    (:A
      _)
    (:B
      _))
  (Development|SetHiddeninGame (Variables|Default|GetPlaceholder) _isa false))

(fn ConstructionScript
  (bind _placeholder (Variables|Default|GetPlaceholder))
  (Components|Box|SetBoxExtent (Variables|Default|GetTrigger) (Variables|Default|Getv_boxExtent) true)
  (Rendering|Components|TextRender|SetText _placeholder (Variables|Default|Getv_placeholderText))
  (Rendering|Components|TextRender|SetTextRenderColor _placeholder (Variables|Default|Getv_placeholderColor))
  (Rendering|Components|TextRender|SetWorldSize _placeholder (Variables|Default|Getv_placeholderSize))
  (Transformation|SetRelativeLocation _placeholder (Variables|Default|Getv_placeholderLocation) false false))