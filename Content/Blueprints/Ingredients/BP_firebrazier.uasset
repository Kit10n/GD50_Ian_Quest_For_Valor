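; Fire brazier hazard that deals environmental damage over time to QuestCharacters inside its DamageRadius.
; Overlap events maintain an array of actors, and an addition at index zero starts a looping one-second timer.
; Each tick damages living characters and attaches a small emitter to their capsule, while removing non-characters and zero-health characters from the array.
; A per-tick hit counter clears the timer when nobody was damaged.
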(event OnComponentBeginOverlap(DamageRadius)
  (params (OverlappedComponent :type Primitive%20Component%20Object%20Reference) (OtherActor :type Actor%20Object%20Reference) (OtherComp :type Primitive%20Component%20Object%20Reference) (OtherBodyIndex :type Integer) (bFromSweep :type Boolean) (SweepResult :type Hit%20Result%20Structure%20%28by%20ref%29))
  (bind _returnvalue (Utilities|Array|Add (Variables|Default|GetV%20Overlapping%20Actors) OtherActor))
  (Math|Integer|CompareInt _returnvalue
    (:==
      (bind _returnvalue_2 (Utilities|Time|SetTimerbyEvent (delegate Custom|DamageOverTime) 1.0 true))
      (Variables|Default|SetV%20Timer _returnvalue_2))))

(event OnComponentEndOverlap(DamageRadius)
  (params (OverlappedComponent :type Primitive%20Component%20Object%20Reference) (OtherActor :type Actor%20Object%20Reference) (OtherComp :type Primitive%20Component%20Object%20Reference) (OtherBodyIndex :type Integer))
  (Utilities|Array|RemoveItem (Variables|Default|GetV%20Overlapping%20Actors) OtherActor))

(event Custom|DamageOverTime
  (for _array_element (Variables|Default|GetV%20Overlapping%20Actors)
    (if (Collision|IsOverlappingActor (Variables|Default|GetDamageRadius) _array_element :!class /Script/Engine.PrimitiveComponent)
      (bind _asquest_character (Utilities|Casting|CastToQuestCharacter _array_element)
        (:then
          (Math|Float|CompareFloat (Variables|/Game/Blueprints/Characters/QuestCharacter.QuestCharacter_C|GetHealth _asquest_character) 0.0
            (:>
              (Game|Damage|ApplyDamage _array_element 2.0 0 0 "/Engine/EngineDamageTypes/DmgTypeBP_Environmental.DmgTypeBP_Environmental_C")
              (Effects|SpawnEmitterAttached 0 (Variables|/Script/Engine.Character|GetCapsuleComponent _asquest_character) "None" "0, 0, 0" "0, 0, 0" "0.200000,0.200000,0.200000")
              (Math|Integer|IncrementInt (Variables|Default|GetV%20Counter)))
            (:==
              (Utilities|Array|RemoveItem (Variables|Default|GetV%20Overlapping%20Actors) _array_element :!label _label))))
        (:CastFailed
          (goto _label)))))
  (Math|Integer|CompareInt (Variables|Default|GetV%20Counter)
    (:>
      _)
    (:==
      (Utilities|Time|ClearandInvalidateTimerbyHandle (Variables|Default|GetV%20Timer))))
  (Variables|Default|SetV%20Counter 0))

(fn ConstructionScript)